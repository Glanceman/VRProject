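; Interactable button actor that toggles on and off to drive a linked triggerable actor.
; Interact plays a click sound and flips the state, yawing the CorePivot by AngleRange.
; Each change calls Trigger with the new state on TriggerableActor through BP_TriggerableInterface.
; ShowInfo reveals the widget and uses a short retriggerable delay to hide it once calls stop.
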(event `TurnOn`
  (bind _triggerableactor (`self.TriggerableActor`))
  (set `self.bOn?` true)
  (`SceneComponent.K2_SetRelativeRotation` (`self.CorePivot`) (`KismetMathLibrary.MakeRotator` 0.0 0.0 (* (`self.AngleRange`) -1.0)) false false)
  (`/Engine/EditorBlueprintResources/StandardMacros.IsValid` _triggerableactor
    (:`Is Valid`
      (bind _asbp_triggerable_interface (cast `/Game/Interface/BP_TriggerableInterface` _triggerableactor))
      (`/Game/Interface/BP_TriggerableInterface.Trigger` _asbp_triggerable_interface true))))

(event `TurnOff`
  (bind _triggerableactor (`self.TriggerableActor`))
  (bind _corepivot (`self.CorePivot`))
  (bind (_relativerotation_roll _relativerotation_pitch _relativerotation_yaw) (`KismetMathLibrary.BreakRotator` (`SceneComponent.RelativeRotation` _corepivot)))
  (set `self.bOn?` false)
  (`SceneComponent.K2_SetRelativeRotation` _corepivot (`KismetMathLibrary.MakeRotator` 0.0 0.0 (+ _relativerotation_yaw (`self.AngleRange`))) false false)
  (`/Engine/EditorBlueprintResources/StandardMacros.IsValid` _triggerableactor
    (:`Is Valid`
      (bind _asbp_triggerable_interface (cast `/Game/Interface/BP_TriggerableInterface` _triggerableactor))
      (`/Game/Interface/BP_TriggerableInterface.Trigger` _asbp_triggerable_interface false))))

(event `/Game/Interface/BP_InteractInterface.Interact`
  (params (InteractComponent :type "PrimitiveComponent Object Reference"))
  (`GameplayStatics.PlaySoundAtLocation` "/Game/Sound/ClickCue.ClickCue" (`self.K2_GetActorLocation`) (struct) 1.0 1.0 0.0 null null null null)
  (if (`self.bOn?`)
    (`self.TurnOff`)
    (else
      (`self.TurnOn`))))

(event `/Game/Interface/BP_WidgetInterface.ShowInfo`
  (bind _widget (`self.Widget`))
  (`SceneComponent.SetHiddenInGame` _widget false false)
  (`KismetSystemLibrary.RetriggerableDelay` 0.2)
  (`SceneComponent.SetHiddenInGame` _widget true false))

(fn `UserConstructionScript`)