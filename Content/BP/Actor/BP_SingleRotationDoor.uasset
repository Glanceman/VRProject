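; BP_SingleRotationDoor is a hinged door actor that swings open and shut through Open and Close events.
; A Timeline plays forward to open and reverses to close.
; Its two alpha tracks separately lerp the CorePivot yaw toward TargetYaw and the HandlePivot pitch toward TargetHandlePitch, so the handle animates alongside the door swing.
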(event `Open`
  (bind (_direction _alpha _alpha2) (`Timeline|Timeline` :!label _label)
    (:`Update`
      (`|ExecutionSequence`
        (:`then_0`
          (`SceneComponent.K2_SetRelativeRotation` (`self.CorePivot`) (`KismetMathLibrary.MakeRotator` 0.0 0.0 (`KismetMathLibrary.Lerp` 0.0 (`self.TargetYaw`) _alpha)) false false))
        (:`then_1`
          (`SceneComponent.K2_SetRelativeRotation` (`self.HandlePivot`) (`KismetMathLibrary.MakeRotator` 0.0 (`KismetMathLibrary.Lerp` 0.0 (`KismetMathLibrary.Conv_IntToDouble` (`self.TargetHandlePitch`)) _alpha2)) false false))))))

(event `Close`
  (goto _label :!via `Reverse`))

(fn `UserConstructionScript`)