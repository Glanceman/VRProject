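; Base Blueprint for an interactable sliding door with two independently operated panels, RightCore and LeftCore.
; BeginPlay stores each panel's relative location, and Interact plays or reverses that panel's timeline based on its moved flag, which toggles when the timeline finishes.
; The timelines lerp relative Y from the stored value to SlidingRange for the right panel and its negative for the left, as absolute targets rather than offsets.
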(event `self.ReceiveBeginPlay`
  (`parent.ReceiveBeginPlay`)
  (`|ExecutionSequence`
    (:`then_0`
      (set `self.OriginalRelativeLocation_RightCore` (`SceneComponent.RelativeLocation` (`self.RightCore`))))
    (:`then_1`
      (set `self.OriginalRelativeLocation_LeftCore` (`SceneComponent.RelativeLocation` (`self.LeftCore`))))))

(event `/Game/Interface/BP_InteractInterface.Interact`
  (params (InteractComponent :type "PrimitiveComponent Object Reference"))
  (bind (_originalrelativelocation_leftcore_x _originalrelativelocation_leftcore_y _originalrelativelocation_leftcore_z) (`KismetMathLibrary.BreakVector` (`self.OriginalRelativeLocation_LeftCore`)))
  (bind (_originalrelativelocation_rightcore_x _originalrelativelocation_rightcore_y _originalrelativelocation_rightcore_z) (`KismetMathLibrary.BreakVector` (`self.OriginalRelativeLocation_RightCore`)))
  (if (== InteractComponent (`self.RightCore`))
    (if (`self.bRightMoved`)
      (bind (_direction _alpha) (`Timeline|Timeline` :!via `Reverse` :!label _label)
        (:`Update`
          (`SceneComponent.K2_SetRelativeLocation` (`self.RightCore`) (`KismetMathLibrary.MakeVector` _originalrelativelocation_rightcore_x (`KismetMathLibrary.Lerp` _originalrelativelocation_rightcore_y (`self.SlidingRange`) _alpha) _originalrelativelocation_rightcore_z) false false))
        (:`Finished`
          (if (`self.bRightMoved`)
            (set `self.bRightMoved` false)
            (else
              (set `self.bRightMoved` true)))))
      (else
        (goto _label)))
    (elif (== InteractComponent (`self.LeftCore`))
      (if (`self.bLeftMoved`)
        (bind (_direction_2 _alpha_2) (`Timeline|Timeline_0` :!via `Reverse` :!label _label_2)
          (:`Update`
            (`SceneComponent.K2_SetRelativeLocation` (`self.LeftCore`) (`KismetMathLibrary.MakeVector` _originalrelativelocation_leftcore_x (`KismetMathLibrary.Lerp` _originalrelativelocation_leftcore_y (* (`self.SlidingRange`) -1.0) _alpha_2) _originalrelativelocation_leftcore_z) false false))
          (:`Finished`
            (if (`self.bLeftMoved`)
              (set `self.bLeftMoved` false)
              (else
                (set `self.bLeftMoved` true)))))
        (else
          (goto _label_2))))))

(fn `UserConstructionScript`
  (`parent.UserConstructionScript`))