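; Base door actor that toggles between open and closed states on interaction and shows an info widget.
; Interact switches on the current state, calls Open or Close, then flips the state; both events are empty here, leaving the actual door behavior undefined.
; ShowInfo unhides the widget and hides it after a short retriggerable delay, so repeated calls keep it visible.
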(event `Open`)

(event `Close`)

(event `/Game/Interface/BP_InteractInterface.Interact`
  (params (InteractComponent :type "PrimitiveComponent Object Reference"))
  (switch `/Game/BP/Actor/Door/E_DoorState` (`self.CurrrentState`)
    (:`NewEnumerator0`
      (`self.Open`)
      (set `self.CurrrentState` "NewEnumerator1"))
    (:`NewEnumerator1`
      (`self.Close`)
      (set `self.CurrrentState` "NewEnumerator0"))))

(event `/Game/Interface/BP_WidgetInterface.ShowInfo`
  (bind _widget (`self.Widget`))
  (`SceneComponent.SetHiddenInGame` _widget false false)
  (`KismetSystemLibrary.RetriggerableDelay` 0.2)
  (`SceneComponent.SetHiddenInGame` _widget true false))

(fn `UserConstructionScript`)