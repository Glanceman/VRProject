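; BP_cabinet is an interactable cabinet actor with two doors that open and close independently.
; BeginPlay caches each pivot's original rotation, and Interact compares the passed component against LeftDoor and RightDoor to toggle that door's open state.
; Each door has its own timeline, played or reversed to lerp its pivot's yaw from the cached value by RotationAmount, mirrored for the left side.
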(event `self.ReceiveBeginPlay`
  (`|ExecutionSequence`
    (:`then_0`
      (set `self.RightOriginalRotation` (`SceneComponent.RelativeRotation` (`self.RightPivot`))))
    (:`then_1`
      (set `self.LeftOriginalRotation` (`SceneComponent.RelativeRotation` (`self.LeftPivot`))))))

(event `/Game/Interface/BP_InteractInterface.Interact`
  (params (InteractComponent :type "PrimitiveComponent Object Reference"))
  (bind (_leftoriginalrotation_roll _leftoriginalrotation_pitch _leftoriginalrotation_yaw) (`KismetMathLibrary.BreakRotator` (`self.LeftOriginalRotation`)))
  (bind (_rightoriginalrotation_roll _rightoriginalrotation_pitch _rightoriginalrotation_yaw) (`KismetMathLibrary.BreakRotator` (`self.RightOriginalRotation`)))
  (if (== InteractComponent (`self.LeftDoor`))
    (if (== (`self.bLeftOpen`) false)
      (set `self.bLeftOpen` true)
      (bind (_direction _alpha) (`Timeline|Timeline` :!label _label)
        (:`Update`
          (`SceneComponent.K2_SetRelativeRotation` (`self.LeftPivot`) (`KismetMathLibrary.MakeRotator` _leftoriginalrotation_roll _leftoriginalrotation_pitch (`KismetMathLibrary.Lerp` _leftoriginalrotation_yaw (+ _leftoriginalrotation_yaw (* (`self.RotationAmount`) -1.0)) _alpha)) false false)))
      (else
        (set `self.bLeftOpen` false)
        (goto _label :!via `Reverse`)))
    (elif (== InteractComponent (`self.RightDoor`))
      (if (== (`self.bRightOpen`) false)
        (set `self.bRightOpen` true)
        (bind (_direction_2 _alpha_2) (`Timeline|Timeline_0` :!label _label_2)
          (:`Update`
            (`SceneComponent.K2_SetRelativeRotation` (`self.RightPivot`) (`KismetMathLibrary.MakeRotator` _rightoriginalrotation_roll _rightoriginalrotation_pitch (`KismetMathLibrary.Lerp` _rightoriginalrotation_yaw (+ _rightoriginalrotation_yaw (`self.RotationAmount`)) _alpha_2)) false false)))
        (else
          (set `self.bRightOpen` false)
          (goto _label_2 :!via `Reverse`))))))

(fn `UserConstructionScript`)