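; BP_WindowBase is a window actor that swings open when the first-person character overlaps it and closes when that overlap ends.
; Actor begin and end overlap events cast to BP_FirstPersonCharacter, then call the Open and Close events.
; These play or reverse a single Timeline, whose alpha lerps the CorePivot component's relative yaw through a quarter turn.
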(event `self.ReceiveActorEndOverlap`
  (params (OtherActor :type "Actor Object Reference"))
  (cast `/Game/FirstPerson/Blueprints/BP_FirstPersonCharacter` OtherActor)
  (`self.Close`))

(event `self.ReceiveActorBeginOverlap`
  (params (OtherActor :type "Actor Object Reference"))
  (cast `/Game/FirstPerson/Blueprints/BP_FirstPersonCharacter` OtherActor)
  (`self.Open`))

(event `Open`
  (bind (_direction _alpha) (`Timeline|Timeline` :!label _label)
    (:`Update`
      (`SceneComponent.K2_SetRelativeRotation` (`self.CorePivot`) (`KismetMathLibrary.MakeRotator` 0.0 0.0 (`KismetMathLibrary.Lerp` 0.0 90.0 _alpha)) false false))))

(event `Close`
  (goto _label :!via `Reverse`))

(fn `UserConstructionScript`)